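; Base character Blueprint that equips a rifle and ties combat events to its animation.
; On BeginPlay it spawns the configured weapon class through a child actor component, caches the rifle and animation Blueprint, then binds rifle attack and health component hurt and death events.
; Hurt and death handlers play the matching animations; death also enables actor collision and notifies the rifle that its owner died.
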(event EventBeginPlay
  (bind _childactorcomponent (Variables|Default|GetChildActorComponent))
  (ChildActorComponent|SetChildActorClass _childactorcomponent (Variables|Default|GetWeaponClass))
  (bind _asbp_base_rifle (Utilities|Casting|CastToBP_BaseRifle (Variables|/Script/Engine.ChildActorComponent|GetChildActor _childactorcomponent))
    (:then
      (Variables|Default|SetRifle _asbp_base_rifle)
      (bind _asabp_character_animation (Utilities|Casting|CastToABP_CharacterAnimation (Components|SkeletalMesh|GetAnimInstance (Variables|Character|GetMesh)))
        (:then
          (Variables|Default|SetAnimationBP _asabp_character_animation)
          (EventDispatchers|BindEventtoOnRifleAttack (Variables|Default|GetRifle) (EventDispatchers|CreateEvent (Variables|Default|GetAnimationBP) :!event FireAnimation))
          (EventDispatchers|BindEventtoOnHurt (Variables|Default|GetAC_HealthComponent) (EventDispatchers|CreateEvent :!event HandleHurt))
          (EventDispatchers|BindEventtoOnDeath (Variables|Default|GetAC_HealthComponent) (EventDispatchers|CreateEvent :!event HandleDeath)))
        (:CastFailed
          (Development|PrintString "Animation cast failed"))))
    (:CastFailed
      (Development|PrintString "A Weapon is needed!"))))

(fn ConstructionScript)

(fn HandleHurt
  (params (Ratio :type Float%20%28double-precision%29))
  (Class|CharacterAnimation|HitAnimation (Variables|Default|GetAnimationBP) Ratio))

(fn HandleDeath
  (params (Ratio :type Float%20%28double-precision%29))
  (Class|CharacterAnimation|DeathAnimation (Variables|Default|GetAnimationBP) Ratio)
  (Collision|SetActorEnableCollision true)
  (Default|OwnerDied (Variables|Default|GetRifle)))