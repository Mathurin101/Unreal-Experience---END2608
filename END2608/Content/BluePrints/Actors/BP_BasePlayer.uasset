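; Base player Blueprint that handles movement, mouse look and attack input.
; Movement follows the control rotation's yaw only, keeping pitch out of forward and strafe directions, while attack input delegates to the Rifle's Attack.
; On BeginPlay it caches the PlayerController and adds a widget to the viewport, or prints an error and destroys itself if the cast fails.
; An unused animation fire call remains disconnected.
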(event EventBeginPlay
  (|CallParentFunction)
  (bind _asplayer_controller (Utilities|Casting|CastToPlayerController (Pawn|GetController))
    (:then
      (Variables|Default|SetPlayerController _asplayer_controller)
      (bind _returnvalue (UserInterface|CreateWidget (Variables|Default|GetClass) (Variables|Default|GetPlayerController)))
      (UserInterface|Viewport|AddtoViewport _returnvalue 0))
    (:CastFailed
      (Development|PrintString "Player Controller was not casted properly")
      (Actor|DestroyActor))))

(event Input|ActionEvents|InputActionAttackInput
  (params (Key :type Key%20Structure :default "None"))
  (:Pressed
    (Default|Attack (Variables|Default|GetRifle))))

(event Input|AxisEvents|InputAxisTurnRight
  (params (AxisValue :type Float%20%28single-precision%29))
  ;[0.15 0.15 0.15 0.5] Mouse Controls
  (Pawn|Input|AddControllerYawInput AxisValue))

(event Input|AxisEvents|InputAxisLookUp
  (params (AxisValue :type Float%20%28single-precision%29))
  ;[0.15 0.15 0.15 0.5] Mouse Controls
  (Pawn|Input|AddControllerPitchInput AxisValue))

(event Input|AxisEvents|InputAxisMoveForward
  (params (AxisValue :type Float%20%28single-precision%29))
  ;[0.15 0.15 0.15 0.5] Movemnet Logic
  (Pawn|Input|AddMovementInput (Math|Vector|GetForwardVector (Math|Rotator|MakeRotator 0.0 0.0 (.Yaw (Math|Rotator|BreakRotator (Pawn|GetControlRotation :!class /Script/Engine.Pawn))))) AxisValue false))

(event Input|AxisEvents|InputAxisStrafe
  (params (AxisValue :type Float%20%28single-precision%29))
  ;[0.15 0.15 0.15 0.5] Movemnet Logic
  (Pawn|Input|AddMovementInput (Math|Vector|GetRightVector (Math|Rotator|MakeRotator 0.0 0.0 (.Yaw (Math|Rotator|BreakRotator (Pawn|GetControlRotation :!class /Script/Engine.Pawn))))) AxisValue false))

(fn ConstructionScript
  (|CallParentFunction))