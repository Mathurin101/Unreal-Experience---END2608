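; Base rifle actor, owned by a parent Pawn, that fires projectiles from a muzzle socket on its skeletal mesh.
; Attack spawns the projectile, broadcasts OnRifleAttack and uses a timer to block refiring; OwnerDied disables shooting.
; Aim comes from a flagged hack: the HUD-owning pawn shoots toward the first WBP_PlayerHUD's destination, while other pawns use their base aim rotation.
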(event Custom|ActionStopped
  (Variables|Default|SetActionHappening false))

(event EventBeginPlay
  (bind _aspawn (Utilities|Casting|CastToPawn (Actor|GetParentActor))
    (:then
      (Variables|Default|SetParent%20Pawn _aspawn))
    (:CastFailed
      (Development|PrintString "Need a Pawn to own this rifle"))))

(fn ConstructionScript)

(fn Attack
  (if (CallFunction|CanShoot)
    (Game|SpawnActorfromClass (Variables|Default|GetProjectileClass) (Math|Transform|MakeTransform (CallFunction|GetSource) (CallFunction|HACKDONOTCONVERTTOCODE) "1.000000,1.000000,1.000000") "Undefined" "MultiplyWithRoot" (Pawn|GetController (Variables|Default|GetParent%20Pawn)) (Variables|Default|GetParent%20Pawn))
    (Variables|Default|SetActionHappening true)
    (Utilities|Time|SetTimerbyEvent (EventDispatchers|CreateEvent :!event Custom|ActionStopped) (Variables|Default|GetRestTimer))
    (Default|CallOnRifleAttack)))

(fn CanShoot
  (return (and (not (Variables|Default|GetActionHappening)) (Variables|Default|GetAlive))))

(fn GetSource
  (return (Transformation|GetSocketLocation (Variables|Default|GetSK_Rifle) (Variables|Default|GetWeaponSocketName))))

(fn HACKDONOTCONVERTTOCODE
  (bind _foundwidgets (Widget|GetAllWidgetsOfClass "/Game/Both/WBP_PlayerHUD.WBP_PlayerHUD_C" true))
  (if (== (Class|UserWidget|GetOwningPlayerPawn (Utilities|Array|Get(acopy) _foundwidgets)) (Variables|Default|GetParent%20Pawn))
    (return (Math|Rotator|MakeRotfromX (- (Class|PlayerHUD|GetDestination (Utilities|Array|Get(acopy) _foundwidgets)) (CallFunction|GetSource))))
    (else
      (return (Pawn|GetBaseAimRotation (Variables|Default|GetParent%20Pawn))))))

(fn OwnerDied
  (Variables|Default|SetAlive false))