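; BP_Projectile is a projectile actor with a sphere collision component and handlers that destroy it on contact.
; The construction script scales the sphere by Size and binds an event to its begin overlap.
; BeginPlay starts a timer of DestroyTime on an event delegate.
; HandleOverlap and HandleHit both just destroy the actor, but the hit binding in the construction script is disconnected and never runs.
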(event EventBeginPlay
  (Utilities|Time|SetTimerbyEvent (EventDispatchers|CreateEvent :!event K2DestroyActor) (Variables|Default|GetDestroyTime)))

(fn ConstructionScript
  (Collision|BindEventtoOnComponentBeginOverlap (Variables|Default|GetSphere%20Collision) (EventDispatchers|CreateEvent :!event HandleOverlap))
  (Transformation|SetWorldScale3D (Variables|Default|GetSphere%20Collision) (Variables|Default|GetSize)))

(fn HandleOverlap
  (params (OverlappedComponent :type Primitive%20Component%20Object%20Reference) (OtherActor :type Actor%20Object%20Reference) (OtherComp :type Primitive%20Component%20Object%20Reference) (OtherBodyIndex :type Integer) (bFromSweep :type Boolean) (SweepResult :type Hit%20Result%20Structure%20%28by%20ref%29))
  (Actor|DestroyActor)
  (return))

(fn HandleHit
  (params (HitComponent :type Primitive%20Component%20Object%20Reference) (OtherActor :type Actor%20Object%20Reference) (OtherComp :type Primitive%20Component%20Object%20Reference) (NormalImpulse :type Vector) (Hit :type Hit%20Result%20Structure%20%28by%20ref%29))
  (Actor|DestroyActor)
  (return))