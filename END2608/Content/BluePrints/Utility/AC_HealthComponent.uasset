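; AC_HealthComponent is an actor component that tracks health for the actor it is attached to.
; On BeginPlay it fills current health to the maximum and binds to the owner's OnTakeAnyDamage event.
; Each hit subtracts the damage, clamps the result between zero and max health, and prints the new value on screen for debugging.
; It has no death handling.
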(event EventBeginPlay
  (Variables|Default|SetCurrentHealth (Variables|Default|GetMaxHealth))
  (EventDispatchers|AssignOnTakeAnyDamage (Components|GetOwner) (EventDispatchers|CreateEvent :!event OnTakeAnyDamage)))

(fn OnTakeAnyDamage
  (params (DamagedActor :type Actor%20Object%20Reference) (Damage :type Float%20%28single-precision%29) (DamageType :type Damage%20Type%20Object%20Reference) (InstigatedBy :type Controller%20Object%20Reference) (DamageCauser :type Actor%20Object%20Reference))
  (bind _output_get (Variables|Default|SetCurrentHealth (Math|Float|Clamp(Float) (- (Variables|Default|GetCurrentHealth) Damage) 0.0 (Variables|Default|GetMaxHealth))))
  (Development|PrintString (Utilities|String|ToString(Float) _output_get) true true "(R=0.922755,G=0.038657,B=1.000000,A=1.000000)" 4.0))